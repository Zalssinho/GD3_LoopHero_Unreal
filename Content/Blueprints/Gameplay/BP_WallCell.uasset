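; BP_WallCell is a gameplay trigger cell that sets a wall in motion when something overlaps its box.
; The first overlap, gated by DoOnce with no reset wired, calls MoveWall on the referenced BPWall without filtering the overlapping actor.
; It also hides the first top-level WBP_Dice widget, then shows it again after a short delay.
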(event OnComponentBeginOverlap(Box)
  (params (OverlappedComponent :type Primitive%20Component%20Object%20Reference) (OtherActor :type Actor%20Object%20Reference) (OtherComp :type Primitive%20Component%20Object%20Reference) (OtherBodyIndex :type Integer) (bFromSweep :type Boolean) (SweepResult :type Hit%20Result%20Structure%20%28by%20ref%29))
  (Utilities|FlowControl|DoOnce false
    (:Completed
      (Default|MoveWall (Variables|Default|GetBP_Wall))
      (bind _foundwidgets (Widget|GetAllWidgetsOfClass "/Game/Blueprints/Widgets/WBP_Dice.WBP_Dice_C" true))
      (Widget|SetVisibility (Utilities|Array|Get(acopy) _foundwidgets) "Hidden")
      (Utilities|FlowControl|Delay 2.0)
      (Widget|SetVisibility (Utilities|Array|Get(acopy) _foundwidgets) "Visible"))))

(event EventBeginPlay
  (|CallParentFunction))

(event Collision|EventActorBeginOverlap
  (params (OtherActor :type Actor%20Object%20Reference))
  (|CallParentFunction OtherActor) ; This node is disabled and will not be called.\nDrag off pins to build functionality.
)

(event EventTick
  (params (DeltaSeconds :type Float%20%28single-precision%29))
  (|CallParentFunction DeltaSeconds) ; This node is disabled and will not be called.\nDrag off pins to build functionality.
)

(fn ConstructionScript
  (|CallParentFunction))