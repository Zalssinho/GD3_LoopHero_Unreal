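; BP_BucheronCell is an interactable that plays a two-part dialogue and rewards its completion with extra remaining time.
; Activate counts interactions, pushes the dialogue component's current row to the pawn's dialogue widget, and starts dialogue only on the first two visits.
; Update steps through rows, then exits: the first visit queues the next part, while the second restarts dialogue, adds hours to GI_Loop's HeureRestante and reveals Cube1.
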(event EventBeginPlay
  (|CallParentFunction)
  (bind _asgi_loop (Utilities|Casting|CastToGI_Loop (Game|GetGameInstance)))
  (Variables|Default|SetAs%20GI%20Loop _asgi_loop))

(event EventActivate
  (params (Pawn :type CBP%20Pawn%20Object%20Reference))
  (bind _bpc_dialoguecomponent (Variables|Default|GetBPC_DialogueComponent))
  (bind _wbp_dialogue (Variables|/Game/Blueprints/Gameplay/CBP_Pawn.CBP_Pawn_C|GetWBP_Dialogue Pawn))
  (Variables|Default|SetNumberOfTime (+ (Variables|Default|GetNumberOfTime) 1))
  (Default|GetCurrentDialogueRowData _bpc_dialoguecomponent)
  (bind _charactername (Default|GetCharacterfromCurrentRow _bpc_dialoguecomponent))
  (bind _dialoguelong (Default|GetDialogueLongfromCurrentRow _bpc_dialoguecomponent))
  (Default|UpdateDialogue _wbp_dialogue _charactername _dialoguelong)
  (if (< (Variables|Default|GetNumberOfTime) 3)
    (Default|StartDialogue _wbp_dialogue)))

(event EventUpdate
  (params (Pawn :type CBP%20Pawn%20Object%20Reference))
  (bind _bpc_dialoguecomponent (Variables|Default|GetBPC_DialogueComponent))
  (bind _wbp_dialogue (Variables|/Game/Blueprints/Gameplay/CBP_Pawn.CBP_Pawn_C|GetWBP_Dialogue Pawn))
  (bind _as_gi_loop (Variables|Default|GetAs%20GI%20Loop))
  (bind _isfinished_ (Default|IsDialogueFinished _bpc_dialoguecomponent))
  (if _isfinished_
    (Default|ExitDialogue _wbp_dialogue)
    (switch int (Variables|Default|GetNumberOfTime)
      (:1
        (Utilities|FlowControl|DoOnce false
          (:Completed
            (Default|NextPartDialogue _bpc_dialoguecomponent))))
      (:2
        (Default|RestartDialogue _bpc_dialoguecomponent)
        (Variables|/Game/Blueprints/Global/GI_Loop.GI_Loop_C|SetHeureRestante _as_gi_loop (+ (Variables|/Game/Blueprints/Global/GI_Loop.GI_Loop_C|GetHeureRestante _as_gi_loop) 5))
        (Rendering|SetVisibility (Variables|Default|GetCube1) true false)))
    (else
      (Default|ReadNextRow _bpc_dialoguecomponent)
      (Default|GetCurrentDialogueRowData _bpc_dialoguecomponent)
      (bind _charactername (Default|GetCharacterfromCurrentRow _bpc_dialoguecomponent))
      (bind _dialoguelong (Default|GetDialogueLongfromCurrentRow _bpc_dialoguecomponent))
      (Default|UpdateDialogue _wbp_dialogue _charactername _dialoguelong))))

(fn ConstructionScript
  (|CallParentFunction))