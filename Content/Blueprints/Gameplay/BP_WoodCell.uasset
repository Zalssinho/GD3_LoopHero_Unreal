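; BP_WoodCell is an interactable actor that starts the lumberjack (Bucheron) minigame and shows dialogue to the activating pawn.
; Activate triggers BP_Bucheron_Manager only once, counts activations, and pushes the current dialogue row to the pawn's dialogue widget, opening it only on the first activation.
; Update advances rows through the dialogue component, then exits the widget when finished and restarts the dialogue if activated just once.
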(event EventBeginPlay
  (|CallParentFunction) ; This node is disabled and will not be called.\nDrag off pins to build functionality.
)

(event Collision|EventActorBeginOverlap
  (params (OtherActor :type Actor%20Object%20Reference))
  (|CallParentFunction OtherActor) ; This node is disabled and will not be called.\nDrag off pins to build functionality.
)

(event EventTick
  (params (DeltaSeconds :type Float%20%28single-precision%29))
  (|CallParentFunction DeltaSeconds) ; This node is disabled and will not be called.\nDrag off pins to build functionality.
)

(event EventUpdate
  (params (Pawn :type CBP%20Pawn%20Object%20Reference))
  (bind _bpc_dialoguecomponent (Variables|Default|GetBPC_DialogueComponent))
  (bind _wbp_dialogue (Variables|/Game/Blueprints/Gameplay/CBP_Pawn.CBP_Pawn_C|GetWBP_Dialogue Pawn))
  (bind _isfinished_ (Default|IsDialogueFinished _bpc_dialoguecomponent))
  (if _isfinished_
    (Default|ExitDialogue _wbp_dialogue)
    (switch int (Variables|Default|GetNumberOfTime)
      (:1
        (Default|RestartDialogue _bpc_dialoguecomponent)))
    (else
      (Default|ReadNextRow _bpc_dialoguecomponent)
      (Default|GetCurrentDialogueRowData _bpc_dialoguecomponent)
      (bind _charactername (Default|GetCharacterfromCurrentRow _bpc_dialoguecomponent))
      (bind _dialoguelong (Default|GetDialogueLongfromCurrentRow _bpc_dialoguecomponent))
      (Default|UpdateDialogue _wbp_dialogue _charactername _dialoguelong))))

(event EventActivate
  (params (Pawn :type CBP%20Pawn%20Object%20Reference))
  (bind _wbp_dialogue (Variables|/Game/Blueprints/Gameplay/CBP_Pawn.CBP_Pawn_C|GetWBP_Dialogue Pawn))
  (bind _bpc_dialoguecomponent (Variables|Default|GetBPC_DialogueComponent))
  (if (Variables|Default|GetMiniGameDone)
    _
    (else
      (bind _returnvalue (Actor|GetActorOfClass "/Game/Blueprints/MiniJeu/BP_Bucheron_Manager.BP_Bucheron_Manager_C"))
      (Default|StartMiniGame _returnvalue)
      (Variables|Default|SetMiniGameDone true)))
  (Variables|Default|SetNumberOfTime (+ (Variables|Default|GetNumberOfTime) 1))
  (Default|GetCurrentDialogueRowData _bpc_dialoguecomponent)
  (bind _charactername (Default|GetCharacterfromCurrentRow _bpc_dialoguecomponent))
  (bind _dialoguelong (Default|GetDialogueLongfromCurrentRow _bpc_dialoguecomponent))
  (Default|UpdateDialogue _wbp_dialogue _charactername _dialoguelong)
  (if (< (Variables|Default|GetNumberOfTime) 2)
    (Default|StartDialogue _wbp_dialogue)))

(fn ConstructionScript
  (|CallParentFunction))