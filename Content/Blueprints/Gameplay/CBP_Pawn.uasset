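; Board-game pawn that stands on Board cells, storing its cell number in the GI_Loop game instance and restoring that position on BeginPlay.
; BeginPlay also creates the dialogue widget, linking it to the dice widget and the pawn.
; Moves ask the Board for the next cell and snap the pawn slightly above it to avoid collisions.
; TryMoving then activates the cell's message, TryMovingOnebyOne just steps once, and UpdateCell refreshes the message.
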(event EventBeginPlay
  (bind _asgi_loop (Utilities|Casting|CastToGI_Loop (Game|GetGameInstance)))
  (Variables|Default|SetBP_Loop_GameInst _asgi_loop)
  (CallFunction|MovetoCell)
  (bind _returnvalue (UserInterface|CreateWidget "/Game/Blueprints/Widgets/WBP_DialogueUI.WBP_DialogueUI_C"))
  (bind _output_get (Variables|Default|SetWBP_Dialogue _returnvalue))
  (Variables|/Game/Blueprints/Widgets/WBP_DialogueUI.WBP_DialogueUI_C|SetWBP_Dice _output_get (Variables|/Game/Blueprints/Gameplay/BP_Dice.BP_Dice_C|GetWidgetDice (Variables|Default|GetDice)))
  (Variables|/Game/Blueprints/Widgets/WBP_DialogueUI.WBP_DialogueUI_C|SetPawn _output_get self)
  (UserInterface|Viewport|AddtoViewport _output_get 0))

(event Collision|EventActorBeginOverlap
  (params (OtherActor :type Actor%20Object%20Reference)))

(event EventTick
  (params (DeltaSeconds :type Float%20%28single-precision%29)))

(fn ConstructionScript)

(fn MovetoCell
  (bind _cell (Default|GetCellbyNumber (Variables|Default|GetBoard) (Variables|/Game/Blueprints/Global/GI_Loop.GI_Loop_C|GetCellNumber (Variables|Default|GetBP_Loop_GameInst))))
  (Transformation|SetActorTransform (Math|Transform|MakeTransform (+ (.location (Transformation|GetActorTransform _cell)) "0.000000,0.000000,6.000000") (.rotation (Transformation|GetActorTransform _cell)) "1.000000,1.000000,1.000000")))

(fn TryMoving
  (params (Value :type Integer))
  (bind _bp_loop_gameinst (Variables|Default|GetBP_Loop_GameInst))
  (bind _cell (Default|GetNextCelltoMove (Variables|Default|GetBoard) (+ Value (Variables|/Game/Blueprints/Global/GI_Loop.GI_Loop_C|GetCellNumber _bp_loop_gameinst))))
  (Variables|/Game/Blueprints/Global/GI_Loop.GI_Loop_C|SetCellNumber _bp_loop_gameinst _cell)
  (CallFunction|MovetoCell)
  (CallFunction|ActivateCell))

(fn TryMovingOnebyOne
  (bind _bp_loop_gameinst (Variables|Default|GetBP_Loop_GameInst))
  (bind _cell (Default|GetNextCelltoMove (Variables|Default|GetBoard) (+ 1 (Variables|/Game/Blueprints/Global/GI_Loop.GI_Loop_C|GetCellNumber _bp_loop_gameinst))))
  (Variables|/Game/Blueprints/Global/GI_Loop.GI_Loop_C|SetCellNumber _bp_loop_gameinst _cell)
  (CallFunction|MovetoCell))

(fn ActivateCell
  (bind _cell (Default|GetCellbyNumber (Variables|Default|GetBoard) (Variables|/Game/Blueprints/Global/GI_Loop.GI_Loop_C|GetCellNumber (Variables|Default|GetBP_Loop_GameInst))))
  (Class|BPIActivable|Activate(Message) _cell self))

(fn UpdateCell
  (bind _cell (Default|GetCellbyNumber (Variables|Default|GetBoard) (Variables|/Game/Blueprints/Global/GI_Loop.GI_Loop_C|GetCellNumber (Variables|Default|GetBP_Loop_GameInst))))
  (Class|BPIActivable|Update(Message) _cell self))