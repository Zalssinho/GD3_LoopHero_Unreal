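; BP_StartCell is a gameplay Blueprint that counts activations and moves the game on to another level.
; Each Activate event increments LoopNumber and opens L_Number2 once the count exceeds one.
; Nothing in this file calls Activate, and the BeginPlay, overlap, Tick and construction graphs add no logic of their own.
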(event EventBeginPlay
  (|CallParentFunction) ; This node is disabled and will not be called.\nDrag off pins to build functionality.
)

(event Collision|EventActorBeginOverlap
  (params (OtherActor :type Actor%20Object%20Reference))
  (|CallParentFunction OtherActor) ; This node is disabled and will not be called.\nDrag off pins to build functionality.
)

(event EventTick
  (params (DeltaSeconds :type Float%20%28single-precision%29))
  (|CallParentFunction DeltaSeconds) ; This node is disabled and will not be called.\nDrag off pins to build functionality.
)

(event EventActivate
  (params (Pawn :type CBP%20Pawn%20Object%20Reference))
  (bind _output_get (Variables|Default|SetLoopNumber (+ (Variables|Default|GetLoopNumber) 1)))
  (if (> _output_get 1)
    (Game|OpenLevel(byObjectReference) "/Game/Maps/L_Number2.L_Number2")))

(fn ConstructionScript
  (|CallParentFunction))