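; BP_ArbreMiniJeu is the clickable tree of the wood minigame, yielding logs.
; A left click on its Box spawns a BP_Buche above the tree's origin with a random horizontal offset, then plays the ShakeArbre timeline.
; The timeline sways the tree by adding sine-based X offsets each update, and CanBeClick blocks further clicks until it finishes.
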(event OnClicked(Box)
  (params (TouchedComponent :type Primitive%20Component%20Object%20Reference) (ButtonPressed :type Key%20Structure))
  (if (== ButtonPressed "LeftMouseButton")
    (if (Variables|Default|GetbCanBeClick)
      (Variables|Default|SetbCanBeClick false)
      (Game|SpawnActorfromClass "/Game/Blueprints/WoodMiniJeu/BP_Buche.BP_Buche_C" (Math|Transform|MakeTransform (+ (Transformation|GetActorLocation) (Math|Vector|MakeVector (Math|Random|RandomFloatinRange -5e+01 5e+01) (Math|Random|RandomFloatinRange -5e+01 5e+01) 1e+02)) "0, 0, 0" "1.000000,1.000000,1.000000") "AlwaysSpawn" "MultiplyWithRoot" 0 0)
      (bind _shake (Timeline|ShakeArbre PlayFromStart)
        (:Update
          (Transformation|AddActorWorldOffset (Math|Vector|MakeVector (* (Math|Trig|Sin(Radians) (Math|Float|MultiplybyPi (* _shake 8.0))) 5.0) 0.0 0.0)))
        (:Finished
          (Variables|Default|SetbCanBeClick true))))))

(fn ConstructionScript)