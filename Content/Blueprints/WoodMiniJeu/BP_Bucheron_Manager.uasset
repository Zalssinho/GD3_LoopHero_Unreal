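; Manager for the lumberjack mini-game, in which the player must reach a target log count within a time limit.
; StartMiniGame hides the dialogue UI, blends the view to this actor, enables click events and creates the HUD.
; MoreBuch increments the count, while TimeOut resets it and restarts the timer, so only success ends the game.
; On success, a short delay precedes returning to a CameraActor view, restoring dialogue and removing the HUD.
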(event Custom|MiniGameOver
  (Variables|Default|SetbActifMiniGame false)
  (Utilities|Time|SetTimerbyEvent (delegate Custom|ReturnGame) 1.5))

(event Custom|ReturnGame
  (bind _refhud (Variables|Default|GetRefHud))
  (bind _refplayercontroller (Variables|Default|GetRefPlayerController))
  (bind _returnvalue (Actor|GetActorOfClass "/Script/Engine.CameraActor"))
  (Game|Player|SetViewTargetwithBlend _refplayercontroller _returnvalue 0.0 "VTBlend_EaseInOut" 0.0 false)
  (Variables|/Script/Engine.PlayerController|SetbShowMouseCursor _refplayercontroller true)
  (Input|SetInputModeGameandUI (Variables|Default|GetRefPlayerController) 0 "DoNotLock" true false)
  (Variables|/Script/Engine.PlayerController|SetbEnableClickEvents (Variables|Default|GetRefPlayerController) false)
  (bind _foundwidgets (Widget|GetAllWidgetsOfClass "/Game/Blueprints/Widgets/WBP_DialogueUI.WBP_DialogueUI_C" true))
  (for _array_element _foundwidgets
    (Widget|SetVisibility _array_element "Visible")
    (Utilities|IsValid _refhud
      (:Is%20Valid
        (Widget|RemovefromParent _refhud)))))

(event Custom|TimeOut
  (bind _output_get (Variables|Default|SetBucheNumber 0))
  (Default|Update (Variables|Default|GetRefHud) _output_get (Variables|Default|GetBuchesObjectif))
  (bind _returnvalue (Utilities|Time|SetTimerbyFunctionName 0 "TimeOut" (Variables|Default|GetLimiteTime)))
  (Variables|Default|SetTimerHandler _returnvalue))

(event EventBeginPlay
  (Variables|Default|SetRefPlayerController (Game|GetPlayerController 0)))

(fn ConstructionScript)

(fn StartMiniGame
  (bind _refplayercontroller (Variables|Default|GetRefPlayerController))
  (Variables|Default|SetbActifMiniGame true)
  (Variables|/Script/Engine.PlayerController|SetbEnableClickEvents (Game|GetPlayerController 0) true)
  (bind _foundwidgets (Widget|GetAllWidgetsOfClass "/Game/Blueprints/Widgets/WBP_DialogueUI.WBP_DialogueUI_C" true))
  (for _array_element _foundwidgets
    (Widget|SetVisibility _array_element "Hidden")
    (Variables|Default|SetBucheNumber 0)
    (Game|Player|SetViewTargetwithBlend _refplayercontroller self 0.0 "VTBlend_EaseInOut" 0.0 false)
    (Variables|/Script/Engine.PlayerController|SetbShowMouseCursor _refplayercontroller true)
    (Input|SetInputModeGameandUI _refplayercontroller 0 "DoNotLock" true false)
    (bind _returnvalue (UserInterface|CreateWidget "/Game/Blueprints/WoodMiniJeu/WBP_Bucheron_HUD.WBP_Bucheron_HUD_C"))
    (bind _output_get (Variables|Default|SetRefHud _returnvalue))
    (UserInterface|Viewport|AddtoViewport _output_get 0)
    (Variables|/Game/Blueprints/WoodMiniJeu/WBP_Bucheron_HUD.WBP_Bucheron_HUD_C|SetRefManager _output_get self)
    (Default|Update _output_get (Variables|Default|GetBucheNumber) (Variables|Default|GetBuchesObjectif))
    (bind _returnvalue_2 (Utilities|Time|SetTimerbyFunctionName 0 "TimeOut" (Variables|Default|GetLimiteTime)))
    (Variables|Default|SetTimerHandler _returnvalue_2)))

(fn MoreBuch
  (bind _output_get (Variables|Default|SetBucheNumber (+ (Variables|Default|GetBucheNumber) 1)))
  (Default|Update (Variables|Default|GetRefHud) _output_get (Variables|Default|GetBuchesObjectif))
  (if (>= (Variables|Default|GetBucheNumber) (Variables|Default|GetBuchesObjectif))
    (Utilities|Time|ClearandInvalidateTimerbyHandle (Variables|Default|GetTimerHandler))
    (CallFunction|MiniGameOver)))