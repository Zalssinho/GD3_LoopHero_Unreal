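; BP_ArbreMiniJeu is a clickable mini-game tree that shakes and drops logs.
; A left click on its Box starts the ShakeArbre timeline and blocks further clicks until it finishes.
; Each timeline update adds a sine-based X offset to the actor and spawns a BP_Buche at a random horizontal position above its origin, so one click yields many logs.
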(event OnClicked(Box)
  (params (TouchedComponent :type Primitive%20Component%20Object%20Reference) (ButtonPressed :type Key%20Structure :default "None"))
  (if (== ButtonPressed "LeftMouseButton")
    (if (Variables|Default|GetbCanBeClick)
      (Variables|Default|SetbCanBeClick false)
      (bind _shake (Timeline|ShakeArbre Play)
        (:Update
          (Transformation|AddActorWorldOffset (Math|Vector|MakeVector (* (Math|Trig|Sin(Radians) (Math|Float|MultiplybyPi (* _shake 8.0))) 5.0) 0.0 0.0))
          (Game|SpawnActorfromClass "/Game/Blueprints/MiniJeu/BP_Buche.BP_Buche_C" (Math|Transform|MakeTransform (+ (Transformation|GetActorLocation) (Math|Vector|MakeVector (Math|Random|RandomFloatinRange -5e+01 5e+01) (Math|Random|RandomFloatinRange -5e+01 5e+01) 1e+02)) "0, 0, 0" "1.000000,1.000000,1.000000") "AlwaysSpawn" "MultiplyWithRoot" 0 0))
        (:Finished
          (Variables|Default|SetbCanBeClick true))))))

(event EventBeginPlay)

(event Collision|EventActorBeginOverlap
  (params (OtherActor :type Actor%20Object%20Reference)))

(event EventTick
  (params (DeltaSeconds :type Float%20%28single-precision%29)))

(fn ConstructionScript)