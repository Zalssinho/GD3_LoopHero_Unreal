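; BP_Bucheron_Manager runs a lumberjack mini-game in which the player reaches a target number of logs.
; StartMiniGame resets the count, blends the view to the manager, shows the cursor and creates the HUD.
; MoreBuch increments the count, updates the HUD and triggers MiniGameOver at the target.
; After a short timer, ReturnGame restores game-only input and removes the HUD, but blends the view to the manager again, not the player.
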(event Custom|MiniGameOver
  (Variables|Default|SetbActifMiniGame false)
  (Development|PrintString "Mini-jeu terminé !")
  (Utilities|Time|SetTimerbyEvent (delegate Custom|ReturnGame) 1.5))

(event Custom|ReturnGame
  (bind _refplayercontroller (Variables|Default|GetRefPlayerController))
  (Game|Player|SetViewTargetwithBlend _refplayercontroller self 0.8 "VTBlend_EaseInOut" 0.0 false)
  (Variables|/Script/Engine.PlayerController|SetbShowMouseCursor _refplayercontroller false)
  (Input|SetInputModeGameOnly _refplayercontroller false)
  (Widget|RemovefromParent (Variables|Default|GetRefHud)))

(event EventBeginPlay
  (Variables|Default|SetRefPlayerController (Game|GetPlayerController 0)))

(fn ConstructionScript)

(fn StartMiniGame
  (bind _refplayercontroller (Variables|Default|GetRefPlayerController))
  (Variables|Default|SetbActifMiniGame true)
  (Variables|Default|SetBucheNumber 0)
  (Game|Player|SetViewTargetwithBlend _refplayercontroller self 0.8 "VTBlend_EaseInOut" 0.0 false)
  (Variables|/Script/Engine.PlayerController|SetbShowMouseCursor _refplayercontroller true)
  (Input|SetInputModeGameandUI _refplayercontroller 0 "DoNotLock" true false)
  (bind _returnvalue (UserInterface|CreateWidget "/Game/Blueprints/MiniJeu/WBP_Bucheron_HUD.WBP_Bucheron_HUD_C"))
  (bind _output_get (Variables|Default|SetRefHud _returnvalue))
  (UserInterface|Viewport|AddtoViewport _output_get 0)
  (Default|Update _output_get (Variables|Default|GetBucheNumber) (Variables|Default|GetBuchesObjectif)))

(fn MoreBuch
  (bind _output_get (Variables|Default|SetBucheNumber (+ (Variables|Default|GetBucheNumber) 1)))
  (Default|Update (Variables|Default|GetRefHud) _output_get (Variables|Default|GetBuchesObjectif))
  (if (>= (Variables|Default|GetBucheNumber) (Variables|Default|GetBuchesObjectif))
    (CallFunction|MiniGameOver)))