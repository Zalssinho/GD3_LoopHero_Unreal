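; Key tracker for the labyrinth mini-game that counts collected keys and ends the game once enough are gathered.
; On BeginPlay it caches every BP_Key actor in the level.
; KeyCollect increments the count and, at three keys, calls EndMiniGame on the labyrinth manager.
; Reset zeroes the count and re-shows the cached keys with collision enabled, so they are reused rather than respawned.
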(event Custom|KeyCollect
  (Variables|Default|SetKeyCount (+ (Variables|Default|GetKeyCount) 1))
  (if (>= (Variables|Default|GetKeyCount) 3)
    (bind _returnvalue (Actor|GetActorOfClass "/Game/Blueprints/LabyrinthMiniJeu/BP_LabyrinthManagerr.BP_LabyrinthManagerr_C"))
    (Default|EndMiniGame _returnvalue)))

(event EventBeginPlay
  (bind _outactors (Actor|GetAllActorsOfClass "/Game/Blueprints/LabyrinthMiniJeu/BP_Key.BP_Key_C"))
  (Variables|Default|SetKeys _outactors))

(fn ConstructionScript)

(fn Reset
  (Variables|Default|SetKeyCount 0)
  (for _array_element (Variables|Default|GetKeys)
    (Rendering|SetActorHiddenInGame _array_element false)
    (Collision|SetActorEnableCollision _array_element true)))