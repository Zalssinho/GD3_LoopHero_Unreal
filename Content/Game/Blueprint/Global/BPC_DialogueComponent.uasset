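; BPC_DialogueComponent is a component that reads dialogue rows from a data table and exposes their contents.
; It looks up a row by converting CurrentRowNumber into a row name, while accessors return the long dialogue text and character from CurrentDialogueRow.
; A negative NewRow on the current row marks the dialogue as finished.
; ReadNextRow is an empty stub and the event graph has no active logic.
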(event EventBeginPlay)

(event EventTick
  (params (DeltaSeconds :type Float%20%28single-precision%29)))

(fn GetCurrentDialogueRowData
  (bind _returnvalue (Utilities|GetDataTableRow (Variables|Default|GetDialogueDatatable) (Utilities|String|StringToName (Utilities|String|ToString(Integer) (Variables|Default|GetCurrentRowNumber))))
    (:then
      (return _returnvalue))))

(fn GetDialogueLongFormCurrentRow
  (return (.DialogueLong (Utilities|Struct|BreakST_DialogueRowDatas (Variables|Default|GetCurrentDialogueRow)))))

(fn GetCharacterFormCurrentRow
  (return (.Character (Utilities|Struct|BreakST_DialogueRowDatas (Variables|Default|GetCurrentDialogueRow)))))

(fn IsDialogueFinished
  (return (< (.NewRow (Utilities|Struct|BreakST_DialogueRowDatas (Variables|Default|GetCurrentDialogueRow))) 0)))

(fn ReadNextRow)