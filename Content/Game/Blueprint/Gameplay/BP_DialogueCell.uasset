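; BP_DialogueCell is an actor that runs a dialogue sequence on a pawn's dialogue widget.
; Its dialogue component supplies the character and long-form line from the current data row.
; Activate pushes that row to the widget and starts the dialogue.
; Each Update call advances to the next row and refreshes the widget, or exits the dialogue once the component reports it finished.
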(event EventBeginPlay
  (|CallParentFunction) ; This node is disabled and will not be called.\nDrag off pins to build functionality.
)

(event Collision|EventActorBeginOverlap
  (params (OtherActor :type Actor%20Object%20Reference))
  (|CallParentFunction OtherActor) ; This node is disabled and will not be called.\nDrag off pins to build functionality.
)

(event EventTick
  (params (DeltaSeconds :type Float%20%28single-precision%29))
  (|CallParentFunction DeltaSeconds) ; This node is disabled and will not be called.\nDrag off pins to build functionality.
)

(event EventActivate
  (params (BP_Pawn :type BP%20Pawn%20Object%20Reference))
  (bind _bpc_dialoguecomponent (Variables|Default|GetBPC_DialogueComponent))
  (bind _widget_dialogue (Variables|/Game/Game/Blueprint/Gameplay/BP_Pawn.BP_Pawn_C|GetWidget%20Dialogue BP_Pawn))
  (Default|GetCurrentDialogueRowData _bpc_dialoguecomponent)
  (bind _charactername (Default|GetCharacterFormCurrentRow _bpc_dialoguecomponent))
  (bind _dialoguelong (Default|GetDialogueLongFormCurrentRow _bpc_dialoguecomponent))
  (Default|UpdateDialogue _widget_dialogue _charactername _dialoguelong)
  (Default|StartDialogue _widget_dialogue))

(event EventUpdate
  (params (Pawn :type BP%20Pawn%20Object%20Reference))
  (bind _bpc_dialoguecomponent (Variables|Default|GetBPC_DialogueComponent))
  (bind _widget_dialogue (Variables|/Game/Game/Blueprint/Gameplay/BP_Pawn.BP_Pawn_C|GetWidget%20Dialogue Pawn))
  (bind _is_finish (Default|IsDialogueFinished _bpc_dialoguecomponent))
  (if _is_finish
    (Default|ExitDialogue _widget_dialogue)
    (else
      (Default|ReadNextRow _bpc_dialoguecomponent)
      (bind _charactername (Default|GetCharacterFormCurrentRow _bpc_dialoguecomponent))
      (bind _dialoguelong (Default|GetDialogueLongFormCurrentRow _bpc_dialoguecomponent))
      (Default|UpdateDialogue _widget_dialogue _charactername _dialoguelong))))

(fn ConstructionScript
  (|CallParentFunction))