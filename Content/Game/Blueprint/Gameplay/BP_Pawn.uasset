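; Board game pawn that occupies numbered cells on a Board.
; Its current cell number lives in BP_LoopGameInstance, and on BeginPlay it snaps to that cell's location and rotation.
; TryMoving adds a value to the cell number, lets the Board resolve the destination, saves it and snaps there.
; TryMovingOneByOne currently has identical logic, with no intermediate steps.
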(event EventBeginPlay
  (bind _asbp_loop_game_instance (Utilities|Casting|CastToBP_LoopGameInstance (Game|GetGameInstance)))
  (Variables|Default|SetBP%20Loop%20Game%20Instance _asbp_loop_game_instance)
  (CallFunction|MovetoCell))

(event Collision|EventActorBeginOverlap
  (params (OtherActor :type Actor%20Object%20Reference)))

(event EventTick
  (params (DeltaSeconds :type Float%20%28single-precision%29)))

(fn ConstructionScript)

(fn MovetoCell
  (bind _cell (Default|GetCellbyNumber (Variables|Default|GetBoard) (Variables|/Game/Game/Blueprint/Global/BP_LoopGameInstance.BP_LoopGameInstance_C|GetCellNumber (Variables|Default|GetBP%20Loop%20Game%20Instance))))
  (Transformation|SetActorLocation (.location (Transformation|GetActorTransform _cell)) false false)
  (Transformation|SetActorRotation (.rotation (Transformation|GetActorTransform _cell))))

(fn TryMoving
  (params (Value :type Integer))
  (bind _bp_loop_game_instance (Variables|Default|GetBP%20Loop%20Game%20Instance))
  (bind _cell (Default|GetNextCelltoMove (Variables|Default|GetBoard) (+ Value (Variables|/Game/Game/Blueprint/Global/BP_LoopGameInstance.BP_LoopGameInstance_C|GetCellNumber _bp_loop_game_instance))))
  (Variables|/Game/Game/Blueprint/Global/BP_LoopGameInstance.BP_LoopGameInstance_C|SetCellNumber _bp_loop_game_instance _cell)
  (CallFunction|MovetoCell))

(fn TryMovingOnebyOne
  (params (Value :type Integer))
  (bind _bp_loop_game_instance (Variables|Default|GetBP%20Loop%20Game%20Instance))
  (bind _cell (Default|GetNextCelltoMove (Variables|Default|GetBoard) (+ Value (Variables|/Game/Game/Blueprint/Global/BP_LoopGameInstance.BP_LoopGameInstance_C|GetCellNumber _bp_loop_game_instance))))
  (Variables|/Game/Game/Blueprint/Global/BP_LoopGameInstance.BP_LoopGameInstance_C|SetCellNumber _bp_loop_game_instance _cell)
  (CallFunction|MovetoCell))